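; StaticTarget is a damageable target that awards a point to the player who destroys it.
; AnyDamage subtracts floored damage from Health and, at zero or below, runs the kill logic only with authority.
; That logic casts the instigator's PlayerState to MyPlayerState, increments its score, then destroys the actor after a short delay.
; No guard blocks further hits during the delay, so each can score again.
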(event `self.ReceiveAnyDamage`
  (params (Damage :type "Float (single-precision)") (DamageType :type "DamageType Object Reference") (InstigatedBy :type "Controller Object Reference") (DamageCauser :type "Actor Object Reference"))
  ;[1 1 1] 被击加分并销毁
  (set `self.Health` (- (`self.Health`) (`KismetMathLibrary.FFloor` Damage)))
  (if (<= (`self.Health`) 0)
    (`/Engine/EditorBlueprintResources/ActorMacros.Switch Has Authority`
      (:`Authority`
        (bind _asmy_player_state (cast `/Game/Blueprints/MyPlayerState` (`Controller.PlayerState` InstigatedBy)))
        (`/Game/Blueprints/MyPlayerState.IncrementScore` _asmy_player_state)
        (`self.DestroySelf`)))))

(event `DestroySelf`
  ;[1 1 1] 被击加分并销毁
  (`KismetSystemLibrary.Delay` 0.2)
  (`self.K2_DestroyActor`))

(fn `UserConstructionScript`)